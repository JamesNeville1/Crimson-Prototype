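; BP_Dog is a companion or enemy dog pawn that chases the player while firing bullets.
; On BeginPlay it caches the player and starts an AIMoveTo follow loop that restarts only on success.
; Tick rotates the mesh toward the player with a -90 yaw offset.
; A Delay in Tick throttles Bullet spawning from the Firearrow's transform to roughly five per second.
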(event Custom|FollowPlayer
  (AI|AIMoveTo self "0, 0, 0" (Variables|Default|GetplayerRef) 1.5e+02 false
    (:OnSuccess
      (CallFunction|FollowPlayer))))

(event EventTick
  (params (DeltaSeconds :type Float%20%28single-precision%29))
  (bind _returnvalue (Transformation|GetActorLocation))
  (bind _playerref (Variables|Default|GetplayerRef))
  (bind _firearrow (Variables|Default|Getfirearrow))
  (bind _returnvalue_2 (Transformation|GetActorLocation _playerref))
  (bind _returnvalue_3 (Math|Rotator|FindLookatRotation _returnvalue _returnvalue_2))
  (Transformation|SetWorldRotation (Variables|Default|GetStaticMesh) (Math|Rotator|MakeRotator (.roll _returnvalue_3) (.pitch _returnvalue_3) (+ (.yaw _returnvalue_3) -9e+01)) false false)
  (Utilities|FlowControl|Delay 0.2)
  (Game|SpawnActorfromClass "/Game/Turret/Bullet.Bullet_C" (Math|Transform|MakeTransform (Transformation|GetWorldLocation _firearrow) (Transformation|GetWorldRotation _firearrow) "1.000000,1.000000,1.000000") "Undefined" "MultiplyWithRoot" 0 0))

(event EventBeginPlay
  (bind _asbp_player (Utilities|Casting|CastToBP_Player (Game|GetPlayerCharacter 0)))
  (Variables|Default|SetplayerRef _asbp_player)
  (CallFunction|FollowPlayer))

(fn ConstructionScript)