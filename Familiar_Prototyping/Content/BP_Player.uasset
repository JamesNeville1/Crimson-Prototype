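; BP_Player is the player character, driven as an active ragdoll that blends physics with looping idle and run animations.
; On BeginPlay, a PhysicalAnimation component applies motor settings below the root bone and simulates those bodies, then the input mapping context is added and the pawn possessed.
; Enhanced Input handles camera-relative movement, look and jump, with move start and completion swapping animations directly on the mesh.
; An unconnected "Grab" print never runs.
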(event Custom|Controls%20Hookup
  (bind _returnvalue (Game|GetPlayerController 0))
  (bind _returnvalue_2 (PlayerController|LocalPlayerSubsystems|GetEnhancedInputLocalPlayerSubsystem _returnvalue))
  ;[1 1 1] Setup
  (Utilities|IsValid _returnvalue_2
    (:Is%20Valid
      (Input|AddMappingContext _returnvalue_2 "/Game/IMC_Default.IMC_Default" 0 "(bIgnoreAllPressedKeysUntilRelease=True,bForceImmediately=False)")
      (Pawn|Possess _returnvalue self))))

(event Custom|Ragdoll%20Hookup
  (bind _mesh (Variables|Character|GetMesh))
  (bind _rootbonename (Variables|Default|GetrootBoneName))
  ;[1 1 1] Setup
  (Class|PhysicalAnimationComponent|SetSkeletalMeshComponent (Variables|Default|GetPhysicalAnimation) (Variables|Character|GetMesh))
  (Class|PhysicalAnimationComponent|ApplyPhysicalAnimationSettingsBelow (Variables|Default|GetPhysicalAnimation) _rootbonename (Utilities|Struct|MakePhysicalAnimationData true 2e+03 3.5e+02 1e+03 3e+02 0.0 1.5e+02) true)
  (Class|SkeletalMeshComponent|SetAllBodiesBelowSimulatePhysics _mesh _rootbonename true false)
  (Class|SkeletalMeshComponent|SetAllBodiesBelowPhysicsBlendWeight _mesh _rootbonename (Variables|Default|GetphysicsBlendWeight) false true)
  (Components|Animation|PlayAnimation (Variables|Character|GetMesh) "/Game/Idle.Idle" true))

(event Input|EnhancedActionEvents|EnhancedInputActionIA_Grab
  (params (ActionValue :type Boolean) (ElapsedSeconds :type Float%20%28double-precision%29) (TriggeredSeconds :type Float%20%28double-precision%29) (InputAction :type Input%20Action%20Object%20Reference :default "/Game/IA_Grab.IA_Grab"))
  ;[1 1 1] Input
)

(event Input|EnhancedActionEvents|EnhancedInputActionIA_Move
  (params (ActionValue :type Vector%202D%20Structure) (ElapsedSeconds :type Float%20%28double-precision%29) (TriggeredSeconds :type Float%20%28double-precision%29) (InputAction :type Input%20Action%20Object%20Reference :default "/Game/IA_Move.IA_Move"))
  (bind _returnvalue (Pawn|GetControlRotation :!class /Script/Engine.Pawn))
  ;[1 1 1] Input
  (:Triggered
    (Pawn|Input|AddMovementInput (Math|Vector|GetForwardVector (Math|Rotator|MakeRotator 0.0 0.0 (.yaw (Pawn|GetControlRotation :!class /Script/Engine.Pawn)))) (.x ActionValue) false)
    (Pawn|Input|AddMovementInput (Math|Vector|GetRightVector (Math|Rotator|MakeRotator (.roll _returnvalue) 0.0 (.yaw _returnvalue))) (.y ActionValue) false))
  (:Started
    (Components|Animation|PlayAnimation (Variables|Character|GetMesh) "/Game/Fast_Run.Fast_Run" true))
  (:Completed
    (Components|Animation|PlayAnimation (Variables|Character|GetMesh) "/Game/Idle.Idle" true)))

(event Input|EnhancedActionEvents|EnhancedInputActionIA_Jump
  (params (ActionValue :type Boolean) (ElapsedSeconds :type Float%20%28double-precision%29) (TriggeredSeconds :type Float%20%28double-precision%29) (InputAction :type Input%20Action%20Object%20Reference :default "/Game/IA_Jump.IA_Jump"))
  ;[1 1 1] Input
  (:Triggered
    (Character|Jump)))

(event Input|EnhancedActionEvents|EnhancedInputActionIA_Look
  (params (ActionValue :type Vector%202D%20Structure) (ElapsedSeconds :type Float%20%28double-precision%29) (TriggeredSeconds :type Float%20%28double-precision%29) (InputAction :type Input%20Action%20Object%20Reference :default "/Game/IA_Look.IA_Look"))
  ;[1 1 1] Input
  (:Triggered
    (Pawn|Input|AddControllerYawInput (.x ActionValue))
    (Pawn|Input|AddControllerPitchInput (.y ActionValue))))

(event EventBeginPlay
  ;[1 1 1] Setup
  (CallFunction|RagdollHookup)
  (CallFunction|ControlsHookup))

(fn ConstructionScript)