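; Player character with Enhanced Input movement, timer-gated shooting, and a melee launch that ends on timer, hit or re-press in an explosion with damage and knockback.
; A physical-animation, blended ragdoll mesh reacts to recoil impulses and goes full physics blend during launches.
; An upgradable stats map, reloaded from the game instance, drives combat values.
; Spawned powerup actors handle upgrades and a bound one-shot powerup; death reloads the level.
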(event OnComponentHit(CapsuleComponent)
  (params (HitComponent :type Primitive%20Component%20Object%20Reference) (OtherActor :type Actor%20Object%20Reference) (OtherComp :type Primitive%20Component%20Object%20Reference) (NormalImpulse :type Vector :default "0, 0, 0") (Hit :type Hit%20Result%20Structure%20%28by%20ref%29))
  ;[0 0.9954 1] James
  (Class|BPIHitable|Hit(Message) OtherActor (.ImpactNormal (Collision|BreakHitResult Hit)))
  (if (Variables|Melee|GetcurrentlyLaunched)
    (CallFunction|EndMeleeLaunchEarly)))

(event Custom|Controls%20Hookup
  (bind _returnvalue (Game|GetPlayerController 0))
  (bind _returnvalue_2 (PlayerController|LocalPlayerSubsystems|GetEnhancedInputLocalPlayerSubsystem _returnvalue))
  ;[0 0.9954 1] James
  ;;[1 1 1] Setup
  (Utilities|IsValid _returnvalue_2
    (:Is%20Valid
      (Input|AddMappingContext _returnvalue_2 "/Game/Player/Input/IMC_Default.IMC_Default" 0 "(bIgnoreAllPressedKeysUntilRelease=True,bForceImmediately=False)")
      (Pawn|Possess _returnvalue self))))

(event Custom|Ragdoll%20Hookup
  (bind _mesh (Variables|Character|GetMesh))
  (bind _rootbonename (Variables|ragdoll|GetrootBoneName))
  ;[0 0.9954 1] James
  ;;[1 1 1] Setup
  (Class|PhysicalAnimationComponent|SetSkeletalMeshComponent (Variables|Default|GetPhysicalAnimation) (Variables|Character|GetMesh))
  (Class|PhysicalAnimationComponent|ApplyPhysicalAnimationSettingsBelow (Variables|Default|GetPhysicalAnimation) _rootbonename (Utilities|Struct|MakePhysicalAnimationData true 2e+03 3.5e+02 1e+03 3e+02 0.0 1.5e+02) true)
  (Class|SkeletalMeshComponent|SetAllBodiesBelowSimulatePhysics _mesh _rootbonename true false)
  (Class|SkeletalMeshComponent|SetAllBodiesBelowPhysicsBlendWeight _mesh _rootbonename (Variables|ragdoll|GetphysicsBlendWeight) false true)
  (Components|Animation|PlayAnimation (Variables|Character|GetMesh) "/Game/Player/Animation/Rifle_Idle.Rifle_Idle" true))

(event Custom|PowerupBinding
  ;[0 0.9954 1] James
  (Default|CallPowerup (.Value (Utilities|Map|Find (Variables|Default|GetpowerupRefs) (Variables|Default|GetcurrentPowerup)))))

(event Custom|Set%20"meleeOnCooldown"%20false
  ;[0 0.9954 1] James
  (Variables|Melee|SetmeleeOnCooldown false))

(event Custom|Set%20"canShoot"%20True
  ;[0 0.9954 1] James
  ;;[1 1 1] Input
  (Variables|gun|SetcanShoot true))

(event Input|EnhancedActionEvents|EnhancedInputActionIA_Shoot
  (params (ActionValue :type Boolean) (ElapsedSeconds :type Float%20%28double-precision%29) (TriggeredSeconds :type Float%20%28double-precision%29) (InputAction :type Input%20Action%20Object%20Reference :default "/Game/Player/Input/IA_Shoot.IA_Shoot"))
  ;[0 0.9954 1] James
  ;;[1 1 1] Input
  (:Triggered
    (if (Variables|gun|GetcanShoot)
      (Variables|gun|SetcanShoot false)
      (CallFunction|SpawnProjectile)
      (CallFunction|AddRecoil)
      (Utilities|Time|SetTimerbyEvent (delegate Custom|Set%20"canShoot"%20True) (.Value (Utilities|Map|Find (Variables|Default|GetplayerUpgradableStats) "NewEnumerator2"))))))

(event Input|EnhancedActionEvents|EnhancedInputActionIA_Move
  (params (ActionValue :type Vector%202D%20Structure) (ElapsedSeconds :type Float%20%28double-precision%29) (TriggeredSeconds :type Float%20%28double-precision%29) (InputAction :type Input%20Action%20Object%20Reference :default "/Game/Player/Input/IA_Move.IA_Move"))
  (bind _returnvalue (Pawn|GetControlRotation :!class /Script/Engine.Pawn))
  ;[0 0.9954 1] James
  ;;[1 1 1] Input
  (:Triggered
    (Pawn|Input|AddMovementInput (Math|Vector|GetForwardVector (Math|Rotator|MakeRotator 0.0 0.0 (.yaw (Pawn|GetControlRotation :!class /Script/Engine.Pawn)))) (* (.x ActionValue) (Variables|movement|GetmoveSpeed)) false)
    (Pawn|Input|AddMovementInput (Math|Vector|GetRightVector (Math|Rotator|MakeRotator (.roll _returnvalue) 0.0 (.yaw _returnvalue))) (* (.y ActionValue) (Variables|movement|GetmoveSpeed)) false))
  (:Started
    (Components|Animation|PlayAnimation (Variables|Character|GetMesh) "/Game/Player/Animation/Rifle_Run.Rifle_Run" true))
  (:Completed
    (Components|Animation|PlayAnimation (Variables|Character|GetMesh) "/Game/Player/Animation/Rifle_Idle.Rifle_Idle" true)))

(event Input|EnhancedActionEvents|EnhancedInputActionIA_Powerup
  (params (ActionValue :type Boolean) (ElapsedSeconds :type Float%20%28double-precision%29) (TriggeredSeconds :type Float%20%28double-precision%29) (InputAction :type Input%20Action%20Object%20Reference :default "/Game/Player/Input/IA_Powerup.IA_Powerup"))
  ;[0 0.9954 1] James
  ;;[1 1 1] Input
  (:Started
    (Default|CallPowerupBound)
    (EventDispatchers|UnbindallEventsfromPowerupBound)))

(event Input|EnhancedActionEvents|EnhancedInputActionIA_Jump
  (params (ActionValue :type Boolean) (ElapsedSeconds :type Float%20%28double-precision%29) (TriggeredSeconds :type Float%20%28double-precision%29) (InputAction :type Input%20Action%20Object%20Reference :default "/Game/Player/Input/IA_Jump.IA_Jump"))
  ;[0 0.9954 1] James
  ;;[1 1 1] Input
  (:Triggered
    (Character|Jump)))

(event Input|EnhancedActionEvents|EnhancedInputActionIA_Look
  (params (ActionValue :type Vector%202D%20Structure) (ElapsedSeconds :type Float%20%28double-precision%29) (TriggeredSeconds :type Float%20%28double-precision%29) (InputAction :type Input%20Action%20Object%20Reference :default "/Game/Player/Input/IA_Look.IA_Look"))
  ;[0 0.9954 1] James
  ;;[1 1 1] Input
  (:Triggered
    (Pawn|Input|AddControllerYawInput (.x ActionValue))))

(event Input|EnhancedActionEvents|EnhancedInputActionIA_Melee
  (params (ActionValue :type Boolean) (ElapsedSeconds :type Float%20%28double-precision%29) (TriggeredSeconds :type Float%20%28double-precision%29) (InputAction :type Input%20Action%20Object%20Reference :default "/Game/Player/Input/IA_Melee.IA_Melee"))
  (bind _currentlylaunched (Variables|Melee|GetcurrentlyLaunched))
  ;[0 0.9954 1] James
  ;;[1 1 1] Input
  (:Started
    (if (not (Variables|Melee|GetmeleeOnCooldown))
      (if (not _currentlylaunched)
        (if (AI|Components|NavMovement|IsFalling (Variables|Character|GetCharacterMovement))
          _
          (else
            (Character|Jump)
            (Utilities|FlowControl|Delay 0.2)))
        (CallFunction|MeleeLaunch)
        (Variables|Melee|SetmeleeOnCooldown true))
      (elif _currentlylaunched
        (CallFunction|EndMeleeLaunchEarly)
        (Development|PrintString "Hello")))))

(event EventBeginPlay
  ;[0 0.9954 1] James
  ;;[1 1 1] Setup
  (CallFunction|RagdollHookup)
  (CallFunction|ControlsHookup)
  (CallFunction|CreatePowerups)
  (Variables|Default|Sethealth (.Value (Utilities|Map|Find (Variables|Default|GetplayerUpgradableStats) "NewEnumerator1")))
  (CallFunction|LoadPreviousData))

(event Game|Damage|EventAnyDamage
  (params (Damage :type Float%20%28single-precision%29) (DamageType :type Damage%20Type%20Object%20Reference) (InstigatedBy :type Controller%20Object%20Reference) (DamageCauser :type Actor%20Object%20Reference))
  ;[0 0.9954 1] James
  (CallFunction|ApplyDamage Damage))

(event EventBindPowerup
  (params (toBind :type BP%20Upgrade%20Starter%20Class%20Reference))
  ;[0 0.9954 1] James
  (Variables|Default|SetcurrentPowerup toBind)
  (EventDispatchers|BindEventtoPowerupBound (delegate Custom|PowerupBinding)))

(event EventUpgradePlayer
  (params (upgrade :type BP%20Upgrade%20Starter%20Class%20Reference))
  ;[0 0.9954 1] James
  (Default|CallPowerup (.Value (Utilities|Map|Find (Variables|Default|GetpowerupRefs) upgrade))))

(fn ConstructionScript)

(fn SpawnProjectile
  (bind _returnvalue (Game|SpawnActorfromClass "/Game/Projectile/Parent/BP_Projectile_Base.BP_Projectile_Base_C" (Math|Transform|MakeTransform (.location (Transformation|GetWorldTransform (Variables|Default|GetShoot%20Point))) (Math|Rotator|MakeRotfromX (Math|Vector|GetForwardVector (Variables|Collision|GetCapsuleComponent))) "1.000000,1.000000,1.000000") "Undefined" "MultiplyWithRoot" 0 0))
  (Default|ProjectileBaseConstructor _returnvalue "IAmPlayerProjectile" (.Value (Utilities|Map|Find (Variables|Default|GetplayerUpgradableStats) "NewEnumerator0"))))

(fn AddRecoil
  (if (not (AI|Components|NavMovement|IsFalling (Variables|Character|GetCharacterMovement)))
    (Physics|AddImpulseatLocation (Variables|Character|GetMesh) (+ (* (* (Math|Vector|GetForwardVector (Variables|Collision|GetCapsuleComponent)) -1.0) (Variables|gun|GetgunRecoil)) (Math|Vector|MakeVector 0.0 0.0 (Variables|gun|GetgunRecoilUp))) (Transformation|GetSocketLocation (Variables|Character|GetMesh) "Head") "Head")))

(fn MeleeLaunch
  (Character|LaunchCharacter "0.000000,0.000000,20000.000000" false false)
  (Character|LaunchCharacter (* (Math|Vector|GetForwardVector (Variables|Collision|GetCapsuleComponent)) (Variables|melee|GetmeleeLaunchVel)) false false)
  (Pawn|Components|CharacterMovement|SetMovementMode (Variables|Character|GetCharacterMovement) "MOVE_Flying" 0)
  (Class|PrimitiveComponent|SetPhysMaterialOverride (Variables|Collision|GetCapsuleComponent) "/Game/Other/PhysicsMat/PHM_No_Friction.PHM_No_Friction")
  (Components|Animation|PlayAnimation (Variables|Character|GetMesh) "/Game/Player/Animation/Hanging_Idle.Hanging_Idle" true)
  (Class|SkeletalMeshComponent|SetAllBodiesBelowPhysicsBlendWeight (Variables|Character|GetMesh) (Variables|ragdoll|GetrootBoneName) 1.0 false true)
  (Variables|Melee|SetcurrentlyLaunched true)
  (bind _returnvalue (Utilities|Time|SetTimerbyEvent (EventDispatchers|CreateEvent :!event EndMeleeLaunch) (Variables|melee|GetlaunchFor)))
  (Variables|Melee|SetlaunchEndTimer _returnvalue))

(fn EndMeleeLaunch
  (bind _explosionpoint (Variables|Default|GetExplosionPoint))
  (bind _returnvalue (Transformation|GetWorldLocation _explosionpoint))
  (Pawn|Components|CharacterMovement|SetMovementMode (Variables|Character|GetCharacterMovement) "MOVE_Walking" 0)
  (Class|PrimitiveComponent|SetPhysMaterialOverride (Variables|Collision|GetCapsuleComponent) "/Game/Other/PhysicsMat/PHM_With_Friction.PHM_With_Friction")
  (Variables|/Script/Engine.MovementComponent|SetVelocity (Variables|Character|GetCharacterMovement) "0, 0, 0")
  (Class|SkeletalMeshComponent|SetAllBodiesBelowPhysicsBlendWeight (Variables|Character|GetMesh) (Variables|ragdoll|GetrootBoneName) (Variables|ragdoll|GetphysicsBlendWeight) false true)
  (Components|Animation|PlayAnimation (Variables|Character|GetMesh) "/Game/Player/Animation/Rifle_Run.Rifle_Run" true)
  (bind _outhits (Class|KismetSystemLibrary|SphereTraceMultibyProfile _returnvalue _returnvalue (.Value (Utilities|Map|Find (Variables|Default|GetplayerUpgradableStats) "NewEnumerator3")) "IAmPlayerProjectile" false 0 "ForOneFrame" true))
  (for _array_element _outhits
    (Game|Damage|ApplyDamage (.HitActor (Collision|BreakHitResult _array_element)) (.Value (Utilities|Map|Find (Variables|Default|GetplayerUpgradableStats) "NewEnumerator5")) 0 0)
    ;[1 1 1] Make interface l8r
    (bind _asbp_ai (Utilities|Casting|CastToBP_AI (.HitActor (Collision|BreakHitResult _array_element))))
    (Physics|AddForce (Variables|/Script/Engine.Character|GetCharacterMovement _asbp_ai) (* (Math|Vector|MakeVector (.X (Math|Vector|BreakVector (Math|Vector|GetUnitDirection(Vector) (Transformation|GetWorldLocation (Variables|/Script/Engine.Character|GetCapsuleComponent _asbp_ai)) (Transformation|GetWorldLocation (Variables|Default|GetExplosionPoint))))) (.Y (Math|Vector|BreakVector (Math|Vector|GetUnitDirection(Vector) (Transformation|GetWorldLocation (Variables|/Script/Engine.Character|GetCapsuleComponent _asbp_ai)) (Transformation|GetWorldLocation (Variables|Default|GetExplosionPoint))))) -0.1) (.Value (Utilities|Map|Find (Variables|Default|GetplayerUpgradableStats) "NewEnumerator6")) -1))
    (Development|PrintString (Utilities|String|ToString(Vector) (* (Math|Vector|MakeVector (.X (Math|Vector|BreakVector (Math|Vector|GetUnitDirection(Vector) (Transformation|GetWorldLocation (Variables|/Script/Engine.Character|GetCapsuleComponent _asbp_ai)) (Transformation|GetWorldLocation (Variables|Default|GetExplosionPoint))))) (.Y (Math|Vector|BreakVector (Math|Vector|GetUnitDirection(Vector) (Transformation|GetWorldLocation (Variables|/Script/Engine.Character|GetCapsuleComponent _asbp_ai)) (Transformation|GetWorldLocation (Variables|Default|GetExplosionPoint))))) -0.1) (.Value (Utilities|Map|Find (Variables|Default|GetplayerUpgradableStats) "NewEnumerator6")) -1))))
  (Variables|Melee|SetcurrentlyLaunched false)
  (Niagara|SpawnSystematLocation "/Game/VFX/NS_explosion.NS_explosion" (Transformation|GetWorldLocation (Variables|Collision|GetCapsuleComponent)))
  (Utilities|Time|SetTimerbyEvent (EventDispatchers|CreateEvent :!event Set"meleeonCooldown"False) (.Value (Utilities|Map|Find (Variables|Default|GetplayerUpgradableStats) "NewEnumerator4"))))

(fn PlayerDie
  (bind _returnvalue (Game|GetCurrentLevelName true))
  (Game|OpenLevel(byName) (Utilities|String|StringToName _returnvalue)))

(fn ApplyDamage
  (params (damage :type Float%20%28double-precision%29))
  (Development|PrintString (Utilities|String|ToString(Boolean) (<= (- (Variables|Default|Gethealth) damage) 0.0)))
  (if (<= (- (Variables|Default|Gethealth) damage) 0.0)
    (CallFunction|PlayerDie))
  (Variables|Default|Sethealth (- (Variables|Default|Gethealth) damage)))

(fn CreatePowerups
  (for _array_element (Variables|Default|GetpowerupsToSpawn)
    (bind _returnvalue (Game|SpawnActorfromClass _array_element (Math|Transform|MakeTransform "0, 0, 0") "Undefined" "MultiplyWithRoot" 0 0))
    (Utilities|Map|Add (Variables|Default|GetpowerupRefs) _array_element _returnvalue)))

(fn EndMeleeLaunchEarly
  (Utilities|Time|ClearandInvalidateTimerbyHandle (Variables|Melee|GetlaunchEndTimer))
  (CallFunction|EndMeleeLaunch))

(fn LoadPreviousData
  (bind _asbp_held_vars (Utilities|Casting|CastToBP_Held_Vars (Game|GetGameInstance)))
  (Variables|Default|SetplayerUpgradableStats (Variables|/Game/BP_Held_Vars.BP_Held_Vars_C|GetplayerUpgradableStats _asbp_held_vars))
  (CallFunction|BindPowerup (Variables|/Game/BP_Held_Vars.BP_Held_Vars_C|Getpowerup _asbp_held_vars)))

(fn OverridePlayerStats
  (params (in :type ENUM_Player_Upgradeables_Keys%20Enum :default "NewEnumerator7") (override :type Float%20%28double-precision%29))
  (Utilities|Map|Remove (Variables|Default|GetplayerUpgradableStats) in)
  (Utilities|Map|Add (Variables|Default|GetplayerUpgradableStats) in override)
  (return))

(fn ReturnMe
  (return self))

(fn ReturnPlayerStats
  (return (Variables|Default|GetplayerUpgradableStats)))