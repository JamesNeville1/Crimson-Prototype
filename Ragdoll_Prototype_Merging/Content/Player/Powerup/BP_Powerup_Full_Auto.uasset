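; Full Auto player powerup that briefly alters two player stats when called, presumably to grant rapid automatic fire.
; CallPowerup increments one stat, caches the current value of another in HoldFloat, then overrides it with a low fixed value.
; A short one-shot timer fires EndPowerup, which removes the increment and restores the cached value.
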(event EventEndPowerup
  (CallFunction|AddtoStat "NewEnumerator0" -1.0)
  (CallFunction|AdjustPlayerStats "NewEnumerator2" (Variables|Default|GetholdFloat)))

(event EventCallPowerup
  (CallFunction|AddtoStat "NewEnumerator0" 1.0)
  (bind _playerstats (CallFunction|ReturnPlayerStats))
  (Variables|Default|SetholdFloat (.Value (Utilities|Map|Find _playerstats "NewEnumerator2")))
  (CallFunction|AdjustPlayerStats "NewEnumerator2" 0.1)
  (Utilities|Time|SetTimerbyEvent (delegate EventEndPowerup) 0.6))

(fn ConstructionScript
  (|CallParentFunction))