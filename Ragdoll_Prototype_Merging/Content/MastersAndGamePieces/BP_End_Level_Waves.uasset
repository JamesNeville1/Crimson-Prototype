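; BP_End_Level_Waves runs enemy waves from BeginPlay and calls OpenDoor once the last wave is cleared.
; A looping timer spawns random EnemyType actors, cycling through Positions until the wave's count is reached.
; Each spawn binds an OnDeath event, and SingleDeathBind decrements the live counter to advance waves.
; The first wave's size comes from QuantityPerWave, but later waves receive the wave index as their size.
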(event Custom|Wave%20Single
  (CallFunction|OnSpawn (.OutItem (Utilities|Array|Random (Variables|Default|GetenemyType))) (.location (Transformation|GetActorTransform (Utilities|Array|Get(acopy) (Variables|Default|Getpositions) (Variables|Default|GetposIndex)))))
  (Development|PrintString "Hello")
  (if (>= (Variables|Default|GetposIndex) (- (Utilities|Array|Length (Variables|Default|Getpositions)) 1))
    (Variables|Default|SetposIndex 0)
    (else
      (Variables|Default|SetposIndex (+ (Variables|Default|GetposIndex) 1))))
  (bind _output_get (Variables|Default|SetenemyData (- (Variables|Default|GetenemyData) 1)))
  (if (<= _output_get 0)
    (Utilities|Time|PauseTimerbyHandle (Variables|Default|GetwaveSingleTimerRef))
    (Variables|Default|SetwaveSingleTimerRef "")
    (Development|PrintString "Hello")))

(event Custom|Wave
  (params (spawnQuant :type Integer))
  (bind _output_get (Variables|Default|SetcurrentWaveCounter spawnQuant))
  (Variables|Default|SetenemyData _output_get)
  (bind _returnvalue (Utilities|Time|SetTimerbyEvent (delegate Custom|Wave%20Single) 0.5 true))
  (Variables|Default|SetwaveSingleTimerRef _returnvalue))

(event EventBeginPlay
  (CallFunction|Wave (Utilities|Array|Get(acopy) (Variables|Default|GetquantityPerWave))))

(fn ConstructionScript
  (|CallParentFunction))

(fn SingleDeathBind
  (bind _output_get (Variables|Default|SetcurrentWaveCounter (- (Variables|Default|GetcurrentWaveCounter) 1)))
  (if (<= _output_get 0)
    (if (>= (Variables|Default|GetcurrentWave) (- (Utilities|Array|Length (Variables|Default|GetquantityPerWave)) 1))
      (CallFunction|OpenDoor)
      (else
        (bind _output_get_2 (Variables|Default|SetcurrentWave (+ 1 (Variables|Default|GetcurrentWave))))
        (CallFunction|Wave _output_get_2)))))

(fn OnSpawn
  (params (type :type BP%20AI%20Class%20Reference) (position :type Vector))
  (bind _returnvalue (Game|SpawnActorfromClass type (Math|Transform|MakeTransform position) "AdjustIfPossibleButAlwaysSpawn" "MultiplyWithRoot" 0 0))
  (EventDispatchers|BindEventtoOnDeath _returnvalue (EventDispatchers|CreateEvent :!event SingleDeathBind)))