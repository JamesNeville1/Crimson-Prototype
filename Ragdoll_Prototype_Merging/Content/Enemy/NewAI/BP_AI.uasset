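; BP_AI is an enemy character that feeds a behavior tree's Blackboard and dies when health runs out.
; Pawn sensing flags when the player is seen, and TriggerPlayerCheck sphere-traces forward to set whether a target is in range.
; Physical animation blends simulated physics below a bone; damage reduces health until OnDeath destroys the actor.
; AttackPlayer only prints, as the montage-based melee hit logic is disconnected.
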(event OnSeePawn(PawnSensing)
  (params (Pawn :type Pawn%20Object%20Reference))
  (Utilities|Casting|CastToBP_Player Pawn)
  (AI|Components|Blackboard|SetValueasBool (AI|GetBlackboard (AI|GetAIController self)) (Utilities|Name|MakeLiteralName "HasSeenPlayer?") true))

(event Custom|AttackPlayer
  (Development|PrintString "ATTACKING"))

(event Custom|Enemy%20Death
  (Actor|DestroyActor))

(event EventBeginPlay
  (bind _bone (Variables|Default|GetBone))
  (Class|PhysicalAnimationComponent|SetSkeletalMeshComponent (Variables|Default|GetPhysicalAnimation) (Variables|Character|GetMesh))
  (Class|PhysicalAnimationComponent|ApplyPhysicalAnimationSettingsBelow (Variables|Default|GetPhysicalAnimation) _bone (Utilities|Struct|MakePhysicalAnimationData true 2e+03 3.5e+02 1e+03 3e+02 0.0 1.5e+02) true)
  (Class|SkeletalMeshComponent|SetAllBodiesBelowSimulatePhysics (Variables|Character|GetMesh) _bone true false)
  (Class|SkeletalMeshComponent|SetAllBodiesBelowPhysicsBlendWeight (Variables|Character|GetMesh) (Variables|Default|GetBone) (Variables|Default|GetragdollBlend) false true)
  (EventDispatchers|BindEventtoOnDeath (delegate Custom|Enemy%20Death)))

(event Game|Damage|EventAnyDamage
  (params (Damage :type Float%20%28single-precision%29) (DamageType :type Damage%20Type%20Object%20Reference) (InstigatedBy :type Controller%20Object%20Reference) (DamageCauser :type Actor%20Object%20Reference))
  ;[0 0.8868 1] James
  (CallFunction|ApplyDamage Damage))

(event EventTriggerPlayerCheck
  (bind _returnvalue (Utilities|Name|MakeLiteralName "InRange?"))
  (bind _returnvalue_2 (Transformation|GetActorLocation))
  (bind _self self)
  (bind _returnvalue_3 (AI|GetAIController _self))
  (bind _returnvalue_4 (AI|GetBlackboard _returnvalue_3))
  ;[0 0.8357 1] James
  (bind _returnvalue_5 (Collision|SphereTraceForObjects _returnvalue_2 (+ _returnvalue_2 (* (Math|Vector|GetForwardVector (Transformation|GetActorRotation)) 1.5e+02)) 6e+01 (Utilities|Array|MakeArray "ObjectTypeQuery7") false 0 "None"))
  (if _returnvalue_5
    (AI|Components|Blackboard|SetValueasBool _returnvalue_4 _returnvalue true)
    (else
      (AI|Components|Blackboard|SetValueasBool _returnvalue_4 _returnvalue false))))

(fn ConstructionScript)

(fn ApplyDamage
  (params (damage :type Float%20%28double-precision%29))
  ;[0 0.8453 1] James
  (Development|PrintString "Hello")
  (if (<= (- (Variables|Default|Gethealth) damage) 0.0)
    (Default|CallOnDeath)
    (else
      (Variables|Default|Sethealth (- (Variables|Default|Gethealth) damage)))))