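; Melee enemy character that detects the player, swings with a baseball-hit montage and is destroyed when its health runs out.
; Sphere overlap shows its health widget and, like taking damage, sets the blackboard's HasSeenPlayer flag.
; AttackPlayer enables the weapon capsule's collision on a timer; a hit deals damage, disables it and clears that flag.
; Physical animation blends partial ragdoll below a bone; an older sphere-trace attack remains unconnected.
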(event OnComponentBeginOverlap(Sphere)
  (params (OverlappedComponent :type Primitive%20Component%20Object%20Reference) (OtherActor :type Actor%20Object%20Reference) (OtherComp :type Primitive%20Component%20Object%20Reference) (OtherBodyIndex :type Integer) (bFromSweep :type Boolean) (SweepResult :type Hit%20Result%20Structure%20%28by%20ref%29))
  (if (== (Utilities|GetClass OtherActor) "/Game/Player/Player/BP_Player.BP_Player_C")
    (CallFunction|SetHasSeen true)
    (Rendering|SetVisibility (Variables|Default|GetWidget) true false)))

(event OnComponentEndOverlap(Sphere)
  (params (OverlappedComponent :type Primitive%20Component%20Object%20Reference) (OtherActor :type Actor%20Object%20Reference) (OtherComp :type Primitive%20Component%20Object%20Reference) (OtherBodyIndex :type Integer))
  (if (== (Utilities|GetClass OtherActor) "/Game/Player/Player/BP_Player.BP_Player_C")
    (Rendering|SetVisibility (Variables|Default|GetWidget) false false)))

(event OnComponentBeginOverlap(WeaponCapsule)
  (params (OverlappedComponent :type Primitive%20Component%20Object%20Reference) (OtherActor :type Actor%20Object%20Reference) (OtherComp :type Primitive%20Component%20Object%20Reference) (OtherBodyIndex :type Integer) (bFromSweep :type Boolean) (SweepResult :type Hit%20Result%20Structure%20%28by%20ref%29))
  ;[0 0.8981 1] Improved Melee - James
  (Game|Damage|ApplyDamage OtherActor 1.0 0 0)
  (Collision|SetCollisionProfileName (Variables|Default|GetWeapon%20Capsule) "NoCollision" true :!class /Script/Engine.PrimitiveComponent)
  (AI|Components|Blackboard|SetValueasBool (AI|GetBlackboard (AI|GetAIController self)) (Utilities|Name|MakeLiteralName "HasSeenPlayer?") false))

(event Custom|AttackPlayer
  ;[0 0.8981 1] Improved Melee - James
  (Animation|PlayAnimMontage "/Game/Enemy/NewNewAI/Baseball_Hit_Anim_mixamo_com_Montage.Baseball_Hit_Anim_mixamo_com_Montage" 1.0 "None")
  (Utilities|Time|SetTimerbyEvent (delegate Custom|Set%20"shouldDamage"%20True) (Variables|Default|GettimeBeforeCanAttack)))

(event Custom|Enemy%20Death
  ;[1 1 1] Ragdoll
  (Actor|DestroyActor))

(event Custom|Set%20"shouldDamage"%20True
  ;[0 0.8981 1] Improved Melee - James
  (Collision|SetCollisionProfileName (Variables|Default|GetWeapon%20Capsule) "IAmEnemyProjectile" true :!class /Script/Engine.PrimitiveComponent))

(event EventBeginPlay
  (bind _bone (Variables|Default|GetBone))
  ;[1 1 1] Ragdoll
  (Variables|Default|Sethealth (Variables|Default|GethealthMax))
  (bind _aswb_enemy_health (Utilities|Casting|CastToWB_Enemy_Health (UserInterface|GetWidget (Variables|Default|GetWidget))))
  (Variables|/Game/WB_Enemy_Health.WB_Enemy_Health_C|SetmyEnemy _aswb_enemy_health self)
  (Utilities|FlowControl|Delay 0.0)
  (Class|PhysicalAnimationComponent|SetSkeletalMeshComponent (Variables|Default|GetPhysicalAnimation) (Variables|Character|GetMesh))
  (Class|PhysicalAnimationComponent|ApplyPhysicalAnimationSettingsBelow (Variables|Default|GetPhysicalAnimation) _bone (Utilities|Struct|MakePhysicalAnimationData true 2e+03 3.5e+02 1e+03 3e+02 0.0 1.5e+02) true)
  (Class|SkeletalMeshComponent|SetAllBodiesBelowSimulatePhysics (Variables|Character|GetMesh) _bone true false)
  (Class|SkeletalMeshComponent|SetAllBodiesBelowPhysicsBlendWeight (Variables|Character|GetMesh) (Variables|Default|GetBone) (Variables|Default|GetragdollBlend) false true)
  (EventDispatchers|BindEventtoOnDeath (delegate Custom|Enemy%20Death))
  (UserInterface|CreateWidget "/Game/WB_Enemy_Health.WB_Enemy_Health_C"))

(event Game|Damage|EventAnyDamage
  (params (Damage :type Float%20%28single-precision%29) (DamageType :type Damage%20Type%20Object%20Reference) (InstigatedBy :type Controller%20Object%20Reference) (DamageCauser :type Actor%20Object%20Reference))
  ;[0 0.8868 1] James
  (CallFunction|ApplyDamage Damage)
  (Audio|PlaySoundatLocation (.OutItem (Utilities|Array|Random (Utilities|Array|MakeArray "/Game/SFX/Blocking_Armor_001.Blocking_Armor_001" "/Game/SFX/Blocking_Armor_002.Blocking_Armor_002" "/Game/SFX/Blocking_Armor_003.Blocking_Armor_003" "/Game/SFX/Blocking_Armor_003.Blocking_Armor_003"))) "0, 0, 0" "0, 0, 0" 1.0 1.0 0.0 0 0 0 0))

(fn ConstructionScript)

(fn ApplyDamage
  (params (damage :type Float%20%28double-precision%29))
  ;[0 0.8453 1] James
  (if (<= (- (Variables|Default|Gethealth) damage) 0.0)
    (Default|CallOnDeath)
    (else
      (Variables|Default|Sethealth (- (Variables|Default|Gethealth) damage))
      (CallFunction|SetHasSeen true))))

(fn SetHasSeen
  (params (param :type Boolean))
  (AI|Components|Blackboard|SetValueasBool (AI|GetBlackboard (AI|GetAIController self)) (Utilities|Name|MakeLiteralName "HasSeenPlayer?") param))