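; End-of-level exit that opens once all enemies are dead and brings in the merchant when its trigger is entered.
; SetupEnemyCounter counts every BP_AI and binds each death to a decrement; at zero, OpenDoor swaps to an emissive material, shows the player's arrow message and plays a sound.
; Overlapping the open box spawns and starts BP_Mechant, destroying all AI if the count is still positive.
; Separate helpers spawn actors and load the next level.
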(event OnComponentBeginOverlap(Box)
  (params (OverlappedComponent :type Primitive%20Component%20Object%20Reference) (OtherActor :type Actor%20Object%20Reference) (OtherComp :type Primitive%20Component%20Object%20Reference) (OtherBodyIndex :type Integer) (bFromSweep :type Boolean) (SweepResult :type Hit%20Result%20Structure%20%28by%20ref%29))
  (if (Variables|Default|GetisOpen)
    (bind _returnvalue (Game|SpawnActorfromClass "/Game/Merchant/BP_Mechant.BP_Mechant_C" (Transformation|GetActorTransform (Variables|Default|GetspawnMerchantAt)) "AlwaysSpawn" "MultiplyWithRoot" 0 0))
    (Default|StartMerchant _returnvalue)
    (Audio|PlaySound2D "/Game/SFX/Task_Accept_Bell_001.Task_Accept_Bell_001" 1.2 1.0 0.0 0 0)
    (if (> (Variables|Default|GetenemyData) 0)
      (bind _outactors (Actor|GetAllActorsOfClass "/Game/Enemy/NewNewAI/BP_AI.BP_AI_C"))
      (for _array_element _outactors
        (Actor|DestroyActor _array_element)))))

(event Custom|Remove%20From%20Data
  (Variables|Default|SetenemyData (- (Variables|Default|GetenemyData) 1))
  (if (<= (Variables|Default|GetenemyData) 0)
    (CallFunction|OpenDoor)))

(event Custom|Manual%20Subscribe
  (params (AI :type BP%20AI%20Object%20Reference))
  (EventDispatchers|BindEventtoOnDeath AI (delegate Custom|Remove%20From%20Data)))

(event Custom|Setup%20Enemy%20Counter
  (bind _outactors (Actor|GetAllActorsOfClass "/Game/Enemy/NewNewAI/BP_AI.BP_AI_C"))
  (Variables|Default|SetenemyData (Utilities|Array|Length _outactors))
  (for _array_element _outactors
    (CallFunction|ManualSubscribe _array_element)))

(fn ConstructionScript)

(fn LoadNextLevel
  (Game|OpenLevel(byName) (Variables|Default|GetnextLevelName)))

(fn OpenDoor
  (Variables|Default|SetisOpen true)
  (Rendering|Material|SetMaterial (Variables|Default|GetStaticMesh) 0 "/Game/Assets/MI_Emissive.MI_Emissive")
  (Class|BPIPlayer|TurnonArrow(Message) (Game|GetPlayerCharacter 0))
  (Audio|PlaySound2D "/Game/SFX/Task_Accept_Ensemble_001.Task_Accept_Ensemble_001" 1.0 1.0 0.0 0 0))

(fn OnSpawn
  (params (type :type BP%20AI%20Class%20Reference) (position :type Vector))
  (bind _returnvalue (Game|SpawnActorfromClass type (Math|Transform|MakeTransform position) "AdjustIfPossibleButAlwaysSpawn" "MultiplyWithRoot" 0 0))
  (return _returnvalue))