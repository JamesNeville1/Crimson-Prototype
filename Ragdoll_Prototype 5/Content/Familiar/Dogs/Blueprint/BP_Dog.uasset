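; BP_Dog is a familiar that follows the player and fires projectiles at the player's last-hit target.
; A self-restarting AI MoveTo keeps it near the player, whether the move succeeds or fails.
; A looping timer turns the mesh toward the target, then spawns a player-profile BP_Projectile_Base from Firearrow after a short delay.
; It only takes a new target from the player's LastHit once the current one is invalid.
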(event Custom|Attack
  (bind _firearrow (Variables|Default|Getfirearrow))
  (Utilities|IsValid (Variables|Default|Gettarget)
    (:Is%20Valid
      (Transformation|SetWorldRotation (Variables|Default|GetStaticMesh) (Math|Rotator|MakeRotator (.roll (Math|Rotator|FindLookatRotation (Transformation|GetActorLocation) (Transformation|GetActorLocation (Variables|Default|Gettarget)))) (.pitch (Math|Rotator|FindLookatRotation (Transformation|GetActorLocation) (Transformation|GetActorLocation (Variables|Default|Gettarget)))) (+ (.yaw (Math|Rotator|FindLookatRotation (Transformation|GetActorLocation) (Transformation|GetActorLocation (Variables|Default|Gettarget)))) -9e+01)) false false)
      (Utilities|FlowControl|Delay 0.2)
      (bind _returnvalue (Game|SpawnActorfromClass "/Game/Projectile/Parent/BP_Projectile_Base.BP_Projectile_Base_C" (Math|Transform|MakeTransform (Transformation|GetWorldLocation _firearrow) (Transformation|GetWorldRotation _firearrow) "1.000000,1.000000,1.000000") "Undefined" "MultiplyWithRoot" 0 0))
      (Default|Setup _returnvalue "IAmPlayerProjectile" 0.6))
    (:Is%20Not%20Valid
      (Variables|Default|Settarget (Variables|/Game/Player/Player/BP_Player.BP_Player_C|GetlastHit (Variables|Default|GetplayerRef))))))

(event Custom|FollowPlayer
  (AI|AIMoveTo self "0, 0, 0" (Variables|Default|GetplayerRef) 1.5e+02 false
    (:OnSuccess
      _)
    (:OnFail
      _))
  (CallFunction|FollowPlayer))

(event EventBeginPlay
  (bind _asbp_player (Utilities|Casting|CastToBP_Player (Game|GetPlayerCharacter 0)))
  (Variables|Default|SetplayerRef _asbp_player)
  (CallFunction|FollowPlayer)
  (Utilities|Time|SetTimerbyEvent (delegate Custom|Attack) 0.2 true))

(fn ConstructionScript)