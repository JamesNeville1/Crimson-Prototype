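; BP_NarrativeBase is a narrative trigger that shows dialogue and moves the game to another level when its box is overlapped.
; Overlap calls StartConversation, which increments TalkIndex and, if in range and no UI exists yet, creates WB_Dialogue with that Dialogue line.
; Timed delays then sequence the widget's black-screen fade, the load of LvlName and a RemoveAllWidgets call.
; The overlap has no actor filter, and an existing widget's text is never updated.
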(event OnComponentBeginOverlap(Box)
  (params (OverlappedComponent :type Primitive%20Component%20Object%20Reference) (OtherActor :type Actor%20Object%20Reference) (OtherComp :type Primitive%20Component%20Object%20Reference) (OtherBodyIndex :type Integer) (bFromSweep :type Boolean) (SweepResult :type Hit%20Result%20Structure%20%28by%20ref%29))
  (bind _ui (Variables|Default|GetUI))
  (CallFunction|StartConversation)
  (Utilities|FlowControl|Delay 0.5)
  (UserInterface|Animation|PlayAnimation _ui (Variables|/Game/UI/Widgets/WB_Dialogue.WB_Dialogue_C|GetFadeBlackScreen _ui) 0.0 1 "Forward" 1.0 false)
  (Widget|SetVisibility (Variables|/Game/UI/Widgets/WB_Dialogue.WB_Dialogue_C|GetBlackScreen _ui) "Visible")
  (Utilities|FlowControl|Delay 2.0)
  (Game|OpenLevel(byName) (Variables|Default|GetlvlName))
  (Utilities|FlowControl|Delay 1.0)
  (Viewport|RemoveAllWidgets))

(event Custom|StartConversation
  ;[1 1 1] Manual Conversations
  (Math|Integer|IncrementInt (Variables|Default|GetTalkIndex)
    (:%20%20
      (if (< (Variables|Default|GetTalkIndex) (Utilities|Array|Length (Variables|Default|GetDialogue)))
        (Variables|Default|GetUI
          (:then)
          (:else
            (bind _returnvalue (UserInterface|CreateWidget "/Game/UI/Widgets/WB_Dialogue.WB_Dialogue_C" (Game|GetPlayerController 0)))
            (bind _output_get (Variables|Default|SetUI _returnvalue))
            (UserInterface|Viewport|AddtoViewport _output_get 0)
            (Rendering|Components|TextRender|SetText (Variables|/Game/UI/Widgets/WB_Dialogue.WB_Dialogue_C|GetDialogueText (Variables|Default|GetUI)) (Utilities|Text|ToText(String) (Utilities|Array|Get(acopy) (Variables|Default|GetDialogue) (Variables|Default|GetTalkIndex))))))))))

(fn ConstructionScript)