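; Base Blueprint for player upgrades, covering both permanent upgrades and temporary powerups.
; Children override the empty CallPowerup event to apply their effect, and EndPowerup is reserved for powerups.
; Helper functions read and override player stats through message calls on player character 0.
; MultiplyStatBy and AddToStat look up a stat by UpgradeID in the stats map and write back the modified value.
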(event Custom|Call%20Powerup
  ;[1 1 1] Overriden by Child, used for upgrades, both permanent and temp powerups
)

(event Custom|End%20Powerup
  ;[1 1 1] Overriden by Child, used for upgrades, both permanent and temp powerups
)

(fn ConstructionScript)

(fn ReturnPlayer
  (bind _me (Class|BPIPlayer|ReturnMe(Message) (Game|GetPlayerCharacter 0)))
  (return _me))

(fn ReturnPlayerStats
  (bind _playerstatscopy (Class|BPIPlayer|ReturnPlayerStats(Message) (Game|GetPlayerCharacter 0)))
  (return _playerstatscopy))

(fn AdjustPlayerStats
  (params (in :type ENUM_Player_Upgradeables_Keys%20Enum :default "NewEnumerator0") (override :type Float%20%28double-precision%29))
  (Class|BPIPlayer|OverridePlayerStats(Message) (Game|GetPlayerCharacter 0) in override))

(fn MultiplyStatby
  (params (upgradeID :type ENUM_Player_Upgradeables_Keys%20Enum :default "NewEnumerator0") (multiplyBy :type Float%20%28double-precision%29))
  (bind _playerstats (Utils|ReturnPlayerStats))
  (Utils|AdjustPlayerStats upgradeID (* multiplyBy (.Value (Utilities|Map|Find _playerstats upgradeID))))
  (return (* multiplyBy (.Value (Utilities|Map|Find _playerstats upgradeID)))))

(fn AddtoStat
  (params (upgradeID :type ENUM_Player_Upgradeables_Keys%20Enum :default "NewEnumerator0") (add :type Float%20%28double-precision%29))
  (bind _playerstats (Utils|ReturnPlayerStats))
  (Utils|AdjustPlayerStats upgradeID (+ add (.Value (Utilities|Map|Find _playerstats upgradeID))))
  (return (+ add (.Value (Utilities|Map|Find _playerstats upgradeID)))))