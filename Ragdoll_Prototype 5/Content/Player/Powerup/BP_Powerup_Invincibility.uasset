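; Invincibility powerup Blueprint that makes the player temporarily invulnerable.
; When called, it gets the player through ReturnPlayer, swaps the first mesh material as a visual cue and sets the Invulnerable flag.
; A short one-shot timer fires EndPowerup, which clears the flag and applies a hardcoded PolygonWar material rather than restoring the cached original.
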(event EventEndPowerup
  (bind _player (CallFunction|ReturnPlayer))
  (Variables|/Game/Player/Player/BP_Player.BP_Player_C|Setinvulnerable _player false)
  (Rendering|Material|SetMaterial (Variables|/Script/Engine.Character|GetMesh _player) 0 "/Game/Assets/WarAssets/PolygonWar/Materials/Mat_PolygonWar_01_A.Mat_PolygonWar_01_A"))

(event EventCallPowerup
  (bind _player (CallFunction|ReturnPlayer))
  (Rendering|Material|SetMaterial (Variables|/Script/Engine.Character|GetMesh _player) 0 "/Game/Assets/WarAssets/WarAsset/Body1.Body1")
  (Variables|/Game/Player/Player/BP_Player.BP_Player_C|Setinvulnerable _player true)
  (Utilities|Time|SetTimerbyEvent (delegate EventEndPowerup) 1.8))

(fn ConstructionScript
  (|CallParentFunction))