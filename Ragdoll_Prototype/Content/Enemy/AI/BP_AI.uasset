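; Enemy AI character that detects the player and runs partial physics-driven animation on its mesh.
; Pawn sensing sets a "HasSeenPlayer?" blackboard key on its AI controller when it sees BP_Player.
; AttackPlayer sphere-traces a short distance forward for pawns and casts the hit to BP_Player, but applies no effect yet.
; On BeginPlay, Physical Animation drives bodies from a chosen bone down, simulating physics only below that bone.
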(event OnSeePawn(PawnSensing)
  (params (Pawn :type Pawn%20Object%20Reference))
  (Utilities|Casting|CastToBP_Player Pawn)
  (AI|Components|Blackboard|SetValueasBool (AI|GetBlackboard (AI|GetAIController self)) (Utilities|Name|MakeLiteralName "HasSeenPlayer?") true))

(event Custom|AttackPlayer
  (bind _returnvalue (Transformation|GetActorLocation))
  (bind (_outhit _returnvalue_2) (Collision|SphereTraceForObjects _returnvalue (+ _returnvalue (* (Math|Vector|GetForwardVector (Transformation|GetActorRotation)) 1.5e+02)) 6e+01 (Utilities|Array|MakeArray "ObjectTypeQuery3") false 0 "ForDuration"))
  (if _returnvalue_2
    (Utilities|Casting|CastToBP_Player (.HitActor (Collision|BreakHitResult _outhit)))))

(event EventBeginPlay
  (bind _bone (Variables|Default|GetBone))
  (Class|PhysicalAnimationComponent|SetSkeletalMeshComponent (Variables|Default|GetPhysicalAnimation) (Variables|Character|GetMesh))
  (Class|PhysicalAnimationComponent|ApplyPhysicalAnimationSettingsBelow (Variables|Default|GetPhysicalAnimation) _bone (Utilities|Struct|MakePhysicalAnimationData true 1e+03 1e+02 1e+03 1e+02 1e+02 1e+02) true)
  (Class|SkeletalMeshComponent|SetAllBodiesBelowSimulatePhysics (Variables|Character|GetMesh) _bone true false))

(fn ConstructionScript)