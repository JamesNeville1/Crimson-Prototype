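; Player character with active-ragdoll movement, projectile shooting and a melee dash.
; PhysicalAnimation blends simulated bodies over directly played animations, while Enhanced Input drives movement, yaw-only look and jumping.
; Shooting runs on a cooldown and adds recoil as a head impulse when grounded.
; Melee launches the character into frictionless flying with full physics blend; a capsule hit notifies the other actor and ends any timed launch with an explosion effect.
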(event OnComponentHit(CapsuleComponent)
  (params (HitComponent :type Primitive%20Component%20Object%20Reference) (OtherActor :type Actor%20Object%20Reference) (OtherComp :type Primitive%20Component%20Object%20Reference) (NormalImpulse :type Vector :default "0, 0, 0") (Hit :type Hit%20Result%20Structure%20%28by%20ref%29))
  (Class|BPIHitable|Hit(Message) OtherActor (.ImpactNormal (Collision|BreakHitResult Hit)))
  (if (Utilities|Time|IsTimerActivebyHandle (Variables|Melee|GetlaunchEndTimer))
    (Utilities|Time|ClearandInvalidateTimerbyHandle (Variables|Melee|GetlaunchEndTimer))
    (CallFunction|EndMeleeLaunch)))

(event Custom|Controls%20Hookup
  (bind _returnvalue (Game|GetPlayerController 0))
  (bind _returnvalue_2 (PlayerController|LocalPlayerSubsystems|GetEnhancedInputLocalPlayerSubsystem _returnvalue))
  ;[1 1 1] Setup
  (Utilities|IsValid _returnvalue_2
    (:Is%20Valid
      (Input|AddMappingContext _returnvalue_2 "/Game/Player/Input/IMC_Default.IMC_Default" 0 "(bIgnoreAllPressedKeysUntilRelease=True,bForceImmediately=False)")
      (Pawn|Possess _returnvalue self))))

(event Custom|Ragdoll%20Hookup
  (bind _mesh (Variables|Character|GetMesh))
  (bind _rootbonename (Variables|ragdoll|GetrootBoneName))
  ;[1 1 1] Setup
  (Class|PhysicalAnimationComponent|SetSkeletalMeshComponent (Variables|Default|GetPhysicalAnimation) (Variables|Character|GetMesh))
  (Class|PhysicalAnimationComponent|ApplyPhysicalAnimationSettingsBelow (Variables|Default|GetPhysicalAnimation) _rootbonename (Utilities|Struct|MakePhysicalAnimationData true 2e+03 3.5e+02 1e+03 3e+02 0.0 1.5e+02) true)
  (Class|SkeletalMeshComponent|SetAllBodiesBelowSimulatePhysics _mesh _rootbonename true false)
  (Class|SkeletalMeshComponent|SetAllBodiesBelowPhysicsBlendWeight _mesh _rootbonename (Variables|ragdoll|GetphysicsBlendWeight) false true)
  (Components|Animation|PlayAnimation (Variables|Character|GetMesh) "/Game/Player/Animation/Rifle_Idle.Rifle_Idle" true))

(event Custom|Timer
  ;[1 1 1] Input
  (Variables|Gun|SetCoolDown false))

(event Custom|SpeedBoost
  (params (Speed :type Float%20%28double-precision%29))
  (Variables|/Script/Engine.CharacterMovementComponent|SetMaxWalkSpeed (Variables|Character|GetCharacterMovement) Speed))

(event Input|EnhancedActionEvents|EnhancedInputActionIA_Shoot
  (params (ActionValue :type Boolean) (ElapsedSeconds :type Float%20%28double-precision%29) (TriggeredSeconds :type Float%20%28double-precision%29) (InputAction :type Input%20Action%20Object%20Reference :default "/Game/Player/Input/IA_Shoot.IA_Shoot"))
  ;[1 1 1] Input
  (:Started
    (if (not (Variables|Gun|GetCoolDown))
      (CallFunction|SpawnProjectile)
      (CallFunction|AddRecoil)
      (Variables|Gun|SetCoolDown true)
      (Utilities|Time|SetTimerbyEvent (delegate Custom|Timer) (Variables|Gun|GetTime)))))

(event Input|EnhancedActionEvents|EnhancedInputActionIA_Move
  (params (ActionValue :type Vector%202D%20Structure) (ElapsedSeconds :type Float%20%28double-precision%29) (TriggeredSeconds :type Float%20%28double-precision%29) (InputAction :type Input%20Action%20Object%20Reference :default "/Game/Player/Input/IA_Move.IA_Move"))
  (bind _returnvalue (Pawn|GetControlRotation :!class /Script/Engine.Pawn))
  ;[1 1 1] Input
  (:Triggered
    (Pawn|Input|AddMovementInput (Math|Vector|GetForwardVector (Math|Rotator|MakeRotator 0.0 0.0 (.yaw (Pawn|GetControlRotation :!class /Script/Engine.Pawn)))) (* (.x ActionValue) (Variables|movement|GetmoveSpeed)) false)
    (Pawn|Input|AddMovementInput (Math|Vector|GetRightVector (Math|Rotator|MakeRotator (.roll _returnvalue) 0.0 (.yaw _returnvalue))) (* (.y ActionValue) (Variables|movement|GetmoveSpeed)) false))
  (:Started
    (Components|Animation|PlayAnimation (Variables|Character|GetMesh) "/Game/Player/Animation/Rifle_Run.Rifle_Run" true))
  (:Completed
    (Components|Animation|PlayAnimation (Variables|Character|GetMesh) "/Game/Player/Animation/Rifle_Idle.Rifle_Idle" true)))

(event Input|EnhancedActionEvents|EnhancedInputActionIA_Jump
  (params (ActionValue :type Boolean) (ElapsedSeconds :type Float%20%28double-precision%29) (TriggeredSeconds :type Float%20%28double-precision%29) (InputAction :type Input%20Action%20Object%20Reference :default "/Game/Player/Input/IA_Jump.IA_Jump"))
  ;[1 1 1] Input
  (:Triggered
    (Character|Jump)))

(event Input|EnhancedActionEvents|EnhancedInputActionIA_Look
  (params (ActionValue :type Vector%202D%20Structure) (ElapsedSeconds :type Float%20%28double-precision%29) (TriggeredSeconds :type Float%20%28double-precision%29) (InputAction :type Input%20Action%20Object%20Reference :default "/Game/Player/Input/IA_Look.IA_Look"))
  ;[1 1 1] Input
  (:Triggered
    (Pawn|Input|AddControllerYawInput (.x ActionValue))))

(event Input|EnhancedActionEvents|EnhancedInputActionIA_Melee
  (params (ActionValue :type Boolean) (ElapsedSeconds :type Float%20%28double-precision%29) (TriggeredSeconds :type Float%20%28double-precision%29) (InputAction :type Input%20Action%20Object%20Reference :default "/Game/Player/Input/IA_Melee.IA_Melee"))
  ;[1 1 1] Input
  (:Started
    (CallFunction|MeleeLaunch)))

(event EventBeginPlay
  ;[1 1 1] Setup
  (CallFunction|RagdollHookup)
  (CallFunction|ControlsHookup))

(fn ConstructionScript)

(fn SpawnProjectile
  (Game|SpawnActorfromClass "/Game/Materials/BP_Projectile_Base.BP_Projectile_Base_C" (Math|Transform|MakeTransform (.location (Transformation|GetWorldTransform (Variables|Default|GetShoot%20Point))) (Math|Rotator|MakeRotfromX (Math|Vector|GetForwardVector (Variables|Collision|GetCapsuleComponent))) "1.000000,1.000000,1.000000") "Undefined" "MultiplyWithRoot" 0 0))

(fn AddRecoil
  (if (not (AI|Components|NavMovement|IsFalling (Variables|Character|GetCharacterMovement)))
    (Physics|AddImpulseatLocation (Variables|Character|GetMesh) (+ (* (* (Math|Vector|GetForwardVector (Variables|Collision|GetCapsuleComponent)) -1.0) (Variables|gun|GetgunRecoil)) (Math|Vector|MakeVector 0.0 0.0 (Variables|gun|GetgunRecoilUp))) (Transformation|GetSocketLocation (Variables|Character|GetMesh) "Head") "Head")))

(fn MeleeLaunch
  (Character|LaunchCharacter "0.000000,0.000000,20000.000000" false false)
  (Character|LaunchCharacter (* (Math|Vector|GetForwardVector (Variables|Collision|GetCapsuleComponent)) (Variables|melee|GetmeleeLaunchVel)) false false)
  (Pawn|Components|CharacterMovement|SetMovementMode (Variables|Character|GetCharacterMovement) "MOVE_Flying" 0)
  (Class|PrimitiveComponent|SetPhysMaterialOverride (Variables|Collision|GetCapsuleComponent) "/Game/Other/PhysicsMat/PHM_No_Friction.PHM_No_Friction")
  (Components|Animation|PlayAnimation (Variables|Character|GetMesh) "/Game/Player/Animation/Hanging_Idle.Hanging_Idle" true)
  (Class|SkeletalMeshComponent|SetAllBodiesBelowPhysicsBlendWeight (Variables|Character|GetMesh) (Variables|ragdoll|GetrootBoneName) 1.0 false true)
  (bind _returnvalue (Utilities|Time|SetTimerbyEvent (EventDispatchers|CreateEvent :!event EndMeleeLaunch) (Variables|melee|GetlaunchFor)))
  (Variables|Melee|SetlaunchEndTimer _returnvalue))

(fn EndMeleeLaunch
  (Development|PrintString "Hello")
  (Pawn|Components|CharacterMovement|SetMovementMode (Variables|Character|GetCharacterMovement) "MOVE_Walking" 0)
  (Class|PrimitiveComponent|SetPhysMaterialOverride (Variables|Collision|GetCapsuleComponent) "/Game/Other/PhysicsMat/PHM_With_Friction.PHM_With_Friction")
  (Variables|/Script/Engine.MovementComponent|SetVelocity (Variables|Character|GetCharacterMovement) "0, 0, 0")
  (Class|SkeletalMeshComponent|SetAllBodiesBelowPhysicsBlendWeight (Variables|Character|GetMesh) (Variables|ragdoll|GetrootBoneName) (Variables|ragdoll|GetphysicsBlendWeight) false true)
  (Components|Animation|PlayAnimation (Variables|Character|GetMesh) "/Game/Player/Animation/Rifle_Run.Rifle_Run" true)
  (Niagara|SpawnSystematLocation "/Game/VFX/NS_explosion.NS_explosion" (Transformation|GetWorldLocation (Variables|Collision|GetCapsuleComponent))))