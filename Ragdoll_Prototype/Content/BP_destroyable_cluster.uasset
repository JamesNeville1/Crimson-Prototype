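; Destroyable cluster actor that breaks apart as a geometry collection when its Hit event is called.
; Hit turns on physics for the geometry collection, then adds velocity-change impulses opposite the normalized hit direction, scaled by a force multiplier, and straight down.
; It then disables the static mesh's collision and prints a debug string.
; The static mesh's component hit event and construction script are empty.
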(event OnComponentHit(StaticMesh)
  (params (HitComponent :type Primitive%20Component%20Object%20Reference) (OtherActor :type Actor%20Object%20Reference) (OtherComp :type Primitive%20Component%20Object%20Reference) (NormalImpulse :type Vector :default "0, 0, 0") (Hit :type Hit%20Result%20Structure%20%28by%20ref%29)))

(event EventHit
  (params (hitDir :type Vector :default "0, 0, 0"))
  (bind _geometrycollection (Variables|Default|GetGeometryCollection))
  (Physics|SetSimulatePhysics (Variables|Default|GetGeometryCollection) true)
  (Physics|AddImpulse _geometrycollection (* (Math|Vector|Normalize hitDir) -1.0 (Variables|Default|GetforceMulti)) "None" true)
  (Physics|AddImpulse _geometrycollection "0.000000,0.000000,-100.000000" "None" true)
  (Collision|SetCollisionEnabled (Variables|Default|GetStaticMesh) "NoCollision")
  (Development|PrintString "Hello"))

(fn ConstructionScript)